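; Base actor for inventory items in the world that players can interact with and pick up.
; BeginInteract caches the controller's inventory component via a message call and, for local controllers only, creates and shows a W_Interactable prompt in the widget component.
; TriggerInteract passes the item to that inventory's PickupItem on authority only.
; The prompt starts hidden and is hidden again on EndInteract.
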(event EventTriggerInteract
  (params (InteractingController :type Player%20Controller%20Object%20Reference) (InteractingMeshComponent :type Skeletal%20Mesh%20Component%20Object%20Reference))
  (Networking|SwitchHasAuthority
    (:Authority
      (Class|InventoryComponent|PickupItem (Variables|Default|GetInteractingInventory) self))))

(event EventBeginInteract
  (params (InteractingController :type Player%20Controller%20Object%20Reference))
  (CallFunction|HandleBeginInteract InteractingController))

(event EventEndInteract
  (Rendering|SetVisibility (Variables|Default|GetInteractableWidget) false false))

(fn ConstructionScript
  (Rendering|SetVisibility (Variables|Default|GetInteractableWidget) false false))

(fn HandleBeginInteract
  (params (InteractingController :type Player%20Controller%20Object%20Reference))
  (bind _interactablewidget (Variables|Default|GetInteractableWidget))
  (bind _output_get (LocalVariables|SetLocalController InteractingController))
  (Utilities|IsValid _output_get
    (:Is%20Valid
      (bind _returnvalue (Class|InventoryInterface|GetInventoryComponent(Message) (LocalVariables|GetLocalController)))
      (Variables|Default|SetInteractingInventory _returnvalue)
      (if (Pawn|IsLocalController (LocalVariables|GetLocalController))
        (bind _returnvalue_2 (UserInterface|CreateWidget "/Game/Blueprints/Game/UI/W_Interactable.W_Interactable_C"))
        (bind _output_get_2 (Variables|Default|SetInteractWidget _returnvalue_2))
        (UserInterface|SetWidget _interactablewidget _output_get_2)
        (Rendering|SetVisibility _interactablewidget true false)))))