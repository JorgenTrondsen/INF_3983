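; Player character Blueprint that handles the HUD overlay, camera switching and modular appearance.
; When locally controlled it creates W_Overlay and broadcasts initial values, after a short timer on clients, while attribute callbacks update health and stamina bars.
; IA_SwitchCam toggles first-person and follow cameras.
; UpdateAppearance applies merged customization meshes and anim class to both body meshes, hiding the first-person neck bone.
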(event Custom|ClientInitDelay
  (Utilities|Time|SetTimerbyEvent (delegate Custom|ClientInitDelayFinished) 1.0))

(event Custom|ClientInitDelayFinished
  (Class|INF3910Character|BroadcastInitialValues))

(event Input|EnhancedActionEvents|EnhancedInputActionIA_SwitchCam
  (params (ActionValue :type Boolean) (ElapsedSeconds :type Float%20%28double-precision%29) (TriggeredSeconds :type Float%20%28double-precision%29) (InputAction :type Input%20Action%20Object%20Reference :default "/Game/Input/Actions/IA_SwitchCam.IA_SwitchCam"))
  (bind _followcamera (Variables|Default|GetFollowCamera))
  (bind _firstpersoncam (Variables|Default|GetFirstPersonCam))
  (Utilities|FlowControl|FlipFlop
    (:A
      (Components|Activation|SetActive _firstpersoncam true false)
      (Components|Activation|SetActive _followcamera false false))
    (:B
      (Components|Activation|SetActive _firstpersoncam false false)
      (Components|Activation|SetActive _followcamera true false))))

(event EventBeginPlay
  (if (Pawn|IsLocallyControlled)
    (Utilities|FlowControl|Sequence
      (:then_0
        (CallFunction|InitOverlay)
        (Networking|SwitchHasAuthority
          (:Authority
            (Class|INF3910Character|BroadcastInitialValues))
          (:Remote
            (CallFunction|ClientInitDelay)))))))

(event EventOnHealthChanged
  (params (CurrentHealth :type Float%20%28single-precision%29) (MaxHealth :type Float%20%28single-precision%29))
  (bind _overlaywidgetref (Variables|Default|GetOverlayWidgetRef))
  (Utilities|IsValid _overlaywidgetref
    (:Is%20Valid
      (Default|SetHealthBar _overlaywidgetref CurrentHealth MaxHealth))))

(event EventOnStaminaChanged
  (params (CurrentStamina :type Float%20%28single-precision%29) (MaxStamina :type Float%20%28single-precision%29))
  (bind _overlaywidgetref (Variables|Default|GetOverlayWidgetRef))
  (Utilities|IsValid _overlaywidgetref
    (:Is%20Valid
      (Default|SetStaminaBar _overlaywidgetref CurrentStamina MaxStamina))))

(fn ConstructionScript)

(fn InitOverlay
  (bind _returnvalue (UserInterface|CreateWidget "/Game/Blueprints/GAS/UI/W_Overlay.W_Overlay_C"))
  (bind _output_get (Variables|Default|SetOverlayWidgetRef _returnvalue))
  (UserInterface|Viewport|AddtoViewport _output_get 0))

(fn UpdateAppearance
  (params (Race :type String) (Gender :type String) (ModelPartSelections :type Model%20Part%20Selection%20Data%20Structure))
  (bind _customizationdata (Variables|Default|GetCustomizationData))
  (bind _mesh (Variables|Character|GetMesh))
  (bind _fp_mesh (Variables|Default|GetFP_Mesh))
  (bind _returnvalue (Class|CustomizationData|MergeModelParts _customizationdata Race Gender ModelPartSelections))
  (bind (_thirdpersonmesh _firstpersonmesh _animblueprint) (Utilities|Struct|BreakMergedMeshes _returnvalue))
  (Class|SkeletalMeshComponent|SetAnimClass _mesh _animblueprint)
  (Components|SkeletalMesh|SetSkeletalMeshAsset _mesh _thirdpersonmesh)
  (Class|SkeletalMeshComponent|SetAnimClass _fp_mesh _animblueprint)
  (Components|SkeletalMesh|SetSkeletalMeshAsset _fp_mesh _firstpersonmesh)
  (Components|SkinnedMesh|HideBonebyName _fp_mesh "bone_EXP_C1_Neck1" "PBO_None"))