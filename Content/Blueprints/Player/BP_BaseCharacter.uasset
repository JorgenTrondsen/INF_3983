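; Base player character with a modular body, a health and stamina overlay, and a first/third-person camera toggle.
; Body parts follow the main mesh's pose via leader pose.
; The locally controlled player creates the overlay, which attribute callbacks update; initial values broadcast immediately on authority, after a short delay on clients.
; Switching cameras swaps head and torso meshes for a first-person torso with its neck bone hidden.
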(event Custom|ClientInitDelay
  (Utilities|Time|SetTimerbyEvent (delegate Custom|ClientInitDelayFinished) 1.0))

(event Custom|ClientInitDelayFinished
  (Class|INF3910Character|BroadcastInitialValues))

(event Input|EnhancedActionEvents|EnhancedInputActionIA_SwitchCam
  (params (ActionValue :type Boolean) (ElapsedSeconds :type Float%20%28double-precision%29) (TriggeredSeconds :type Float%20%28double-precision%29) (InputAction :type Input%20Action%20Object%20Reference :default "/Game/Input/Actions/IA_SwitchCam.IA_SwitchCam"))
  (bind _torso_fp (Variables|Default|GetTorso_FP))
  (bind _firstpersoncam (Variables|Default|GetFirstPersonCam))
  (bind _followcamera (Variables|Default|GetFollowCamera))
  (Utilities|FlowControl|FlipFlop
    (:A
      (Components|Activation|SetActive _firstpersoncam true false)
      (Components|Activation|SetActive _followcamera false false)
      (Development|SetHiddeninGame (Variables|Default|GetFace) true false)
      (Rendering|SetVisibility _torso_fp true false))
    (:B
      (Components|Activation|SetActive _firstpersoncam false false)
      (Components|Activation|SetActive _followcamera true false)
      (Development|SetHiddeninGame (Variables|Default|GetEyes) false false)
      (Rendering|SetVisibility _torso_fp false false))))

(event EventBeginPlay
  (if (Pawn|IsLocallyControlled)
    (CallFunction|InitOverlay)
    (Networking|SwitchHasAuthority
      (:Authority
        (Class|INF3910Character|BroadcastInitialValues))
      (:Remote
        (CallFunction|ClientInitDelay)))))

(event EventOnHealthChanged
  (params (CurrentHealth :type Float%20%28single-precision%29) (MaxHealth :type Float%20%28single-precision%29))
  (bind _overlaywidgetref (Variables|Default|GetOverlayWidgetRef))
  (Utilities|IsValid _overlaywidgetref
    (:Is%20Valid
      (Default|SetHealthBar _overlaywidgetref CurrentHealth MaxHealth))))

(event EventOnStaminaChanged
  (params (CurrentStamina :type Float%20%28single-precision%29) (MaxStamina :type Float%20%28single-precision%29))
  (bind _overlaywidgetref (Variables|Default|GetOverlayWidgetRef))
  (Utilities|IsValid _overlaywidgetref
    (:Is%20Valid
      (Default|SetStaminaBar _overlaywidgetref CurrentStamina MaxStamina))))

(fn ConstructionScript
  (Components|SkinnedMesh|SetLeaderPoseComponent (Variables|Default|GetEars) (Variables|Character|GetMesh) false false)
  (Components|SkinnedMesh|HideBonebyName (Variables|Default|GetTorso_FP) "bone_EXP_C1_Neck1" "PBO_None"))

(fn InitOverlay
  (bind _returnvalue (UserInterface|CreateWidget "/Game/Blueprints/GAS/UI/W_Overlay.W_Overlay_C"))
  (bind _output_get (Variables|Default|SetOverlayWidgetRef _returnvalue))
  (UserInterface|Viewport|AddtoViewport _output_get 0))