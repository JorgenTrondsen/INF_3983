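; Interactable NPC character that shows an interact prompt and runs a dialogue with the local player.
; Triggering interaction creates the dialogue widget, turns the NPC toward the player and binds the widget's exit and talking events.
; Talk montages are picked randomly by race and gender from an anim data asset, with long talks re-rolled on completion.
; Exiting removes the widget, restores game-only input and stops facing the player.
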(event Custom|ExitDialogue
  (CallFunction|HandleExitDialogue (stale EventTriggerInteract InteractingController)))

(event Custom|StartTalking
  (bind _npcappearancedata (Variables|Default|GetNPCAppearanceData))
  (bind (_race _gender) (Utilities|Struct|BreakModelPartSelectionData _npcappearancedata))
  (Animation|Montage|PlayMontage (Variables|Character|GetMesh) (.OutItem (Utilities|Array|Random (Class|AnimData|GetMontages (Variables|Default|GetAnimDataAsset) _race _gender "TalkLong"))) :!label _label
    (:OnCompleted
      (goto _label))))

(event Custom|StopTalking
  (bind _npcappearancedata (Variables|Default|GetNPCAppearanceData))
  (bind (_race _gender) (Utilities|Struct|BreakModelPartSelectionData _npcappearancedata))
  (Animation|StopAnimMontage (.OutItem (Utilities|Array|Random (Class|AnimData|GetMontages (Variables|Default|GetAnimDataAsset) _race _gender "TalkLong")))))

(event EventBeginInteract
  (params (InteractingController :type Player%20Controller%20Object%20Reference))
  (CallFunction|HandleBeginInteract InteractingController))

(event EventTriggerInteract
  (params (InteractingController :type Player%20Controller%20Object%20Reference))
  (bind _npcappearancedata (Variables|Default|GetNPCAppearanceData))
  (bind (_race _gender) (Utilities|Struct|BreakModelPartSelectionData _npcappearancedata))
  (if (Pawn|IsLocalController InteractingController)
    (bind _returnvalue (UserInterface|CreateWidget "/Game/Blueprints/Character/NPC/W_Dialogue.W_Dialogue_C" InteractingController))
    (bind _output_get (Variables|Default|SetDialogueWidget _returnvalue))
    (Class|NPCharacter|CreateDialogueWidget InteractingController _output_get)
    (Class|NPCharacter|FacePlayer InteractingController)
    (Animation|PlayAnimMontage (.OutItem (Utilities|Array|Random (Class|AnimData|GetMontages (Variables|Default|GetAnimDataAsset) _race _gender "Talk"))) 1.0 "None")
    (Variables|Default|SetbIsInDialogue true)
    (EventDispatchers|BindEventtoExitDialogue (Variables|Default|GetDialogueWidget) (delegate Custom|ExitDialogue))
    (EventDispatchers|BindEventtoStartTalking (Variables|Default|GetDialogueWidget) (delegate Custom|StartTalking))
    (EventDispatchers|BindEventtoStopTalking (Variables|Default|GetDialogueWidget) (delegate Custom|StopTalking))))

(event EventEndInteract
  (Rendering|SetVisibility (Variables|Default|GetInteractableWidget) false false))

(fn ConstructionScript
  (Rendering|SetVisibility (Variables|Default|GetInteractableWidget) false false))

(fn HandleBeginInteract
  (params (InteractingController :type Player%20Controller%20Object%20Reference))
  (bind _interactablewidget (Variables|Default|GetInteractableWidget))
  (bind _output_get (LocalVariables|SetLocalController InteractingController))
  (Utilities|IsValid _output_get
    (:Is%20Valid
      (if (Pawn|IsLocalController (LocalVariables|GetLocalController))
        (bind _returnvalue (UserInterface|CreateWidget "/Game/Blueprints/Game/UI/W_Interactable.W_Interactable_C"))
        (bind _output_get_2 (Variables|Default|SetInteractWidget _returnvalue))
        (UserInterface|SetWidget _interactablewidget _output_get_2)
        (Rendering|SetVisibility _interactablewidget true false)))))

(fn HandleExitDialogue
  (params (InteractingController :type Player%20Controller%20Object%20Reference))
  (Widget|RemovefromParent (Variables|Default|GetDialogueWidget))
  (Input|SetInputModeGameOnly InteractingController false)
  (Variables|/Script/Engine.PlayerController|SetbShowMouseCursor InteractingController false)
  (EventDispatchers|UnbindallEventsfromExitDialogue (Variables|Default|GetDialogueWidget))
  (Class|NPCharacter|StopFacingPlayer))