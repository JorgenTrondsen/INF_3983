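; Player character Blueprint that manages a health and stamina HUD and switching between first-person and follow cameras.
; On BeginPlay, the locally controlled pawn creates the overlay widget and broadcasts initial values, immediately with authority or after a short timer on remote clients.
; Health and stamina change events update the overlay bars when the widget is valid.
; First-person is the starting camera, and the IA_SwitchCam input toggles cameras through a FlipFlop.
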(event Custom|ClientInitDelay
  (Utilities|Time|SetTimerbyEvent (delegate Custom|ClientInitDelayFinished) 1.0))

(event Custom|ClientInitDelayFinished
  (Class|BaseCharacter|BroadcastInitialValues))

(event Input|EnhancedActionEvents|EnhancedInputActionIA_SwitchCam
  (params (ActionValue :type Boolean) (ElapsedSeconds :type Float%20%28double-precision%29) (TriggeredSeconds :type Float%20%28double-precision%29) (InputAction :type Input%20Action%20Object%20Reference :default "/Game/Input/Actions/IA_SwitchCam.IA_SwitchCam"))
  (bind _fp_camera (Variables|Default|GetFP_Camera))
  (bind _followcamera (Variables|Default|GetFollowCamera))
  (Utilities|FlowControl|FlipFlop
    (:A
      (Components|Activation|SetActive _fp_camera true false)
      (Components|Activation|SetActive _followcamera false false))
    (:B
      (Components|Activation|SetActive _fp_camera false false)
      (Components|Activation|SetActive _followcamera true false))))

(event EventBeginPlay
  (Utilities|FlowControl|Sequence
    (:then_0
      (if (Pawn|IsLocallyControlled)
        (CallFunction|InitOverlay)
        (Networking|SwitchHasAuthority
          (:Authority
            (Class|BaseCharacter|BroadcastInitialValues))
          (:Remote
            (CallFunction|ClientInitDelay)))))
    (:then_1
      (Components|Activation|SetActive (Variables|Default|GetFP_Camera) true false)
      (Components|Activation|SetActive (Variables|Default|GetFollowCamera) false false))))

(event EventOnHealthChanged
  (params (CurrentHealth :type Float%20%28single-precision%29) (MaxHealth :type Float%20%28single-precision%29))
  (bind _overlaywidgetref (Variables|Default|GetOverlayWidgetRef))
  (Utilities|IsValid _overlaywidgetref
    (:Is%20Valid
      (Default|SetHealthBar _overlaywidgetref CurrentHealth MaxHealth))))

(event EventOnStaminaChanged
  (params (CurrentStamina :type Float%20%28single-precision%29) (MaxStamina :type Float%20%28single-precision%29))
  (bind _overlaywidgetref (Variables|Default|GetOverlayWidgetRef))
  (Utilities|IsValid _overlaywidgetref
    (:Is%20Valid
      (Default|SetStaminaBar _overlaywidgetref CurrentStamina MaxStamina))))

(fn ConstructionScript)

(fn InitOverlay
  (bind _returnvalue (UserInterface|CreateWidget "/Game/Blueprints/Game/UI/W_Overlay.W_Overlay_C"))
  (bind _output_get (Variables|Default|SetOverlayWidgetRef _returnvalue))
  (UserInterface|Viewport|AddtoViewport _output_get 0))