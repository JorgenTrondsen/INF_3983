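; Gameplay ability that fires a projectile, then plays a reload before ending.
; Activation requires the Aiming tag on authority only; non-authority instances fire unchecked.
; Random race/gender-specific fire and reload montages play in sequence, with SpawnProjectile and the fire cue at fire start and a delayed reload cue.
; Ability end cleans up montage tasks, stopping the fire task only if a reload task is valid.
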(event Ability|EventActivateAbility
  (bind _returnvalue (Ability|GetAvatarActorfromActorInfo))
  (bind _returnvalue_2 (Ability|GetAvatarActorfromActorInfo))
  (bind _owningplayerstate (Variables|Default|GetOwningPlayerState))
  (bind _animdataasset (Variables|Default|GetAnimDataAsset))
  (bind _modelpartselectiondata (Variables|/Script/INF_3910.INFPlayerState|GetModelPartSelectionData _owningplayerstate))
  (bind (_race _gender) (Utilities|Struct|BreakModelPartSelectionData _modelpartselectiondata))
  (Ability|HasAuthority
    (:True
      (if (Class|INFAbilitySystemComponent|IsTagActive (Variables|Default|GetOwningASC) "(TagName=\"Player.State.Aiming\")")
        (bind _asynctaskproxy (|PlayMontageandWaitProxy "None" (.OutItem (Utilities|Array|Random (Class|AnimData|GetMontages _animdataasset _race _gender "GunFire"))) 1.0 "None" true 1.0 0.0 false :!label _label)
          (:then
            (Variables|Default|SetAsync%20Task%20Fire _asynctaskproxy)
            (Class|GameplayAbility|ExecuteGameplayCuewithParams (Utilities|Struct|BreakProjectileParams (Variables|Default|GetCurrentProjectileParams)) (Ability|GameplayCue|MakeGameplayCueParameters :Instigator _returnvalue_2 :EffectCauser _returnvalue_2))
            (Class|ProjectileAbility|SpawnProjectile))
          (:OnCompleted
            (bind _asynctaskproxy_2 (|PlayMontageandWaitProxy "None" (.OutItem (Utilities|Array|Random (Class|AnimData|GetMontages _animdataasset _race _gender "GunReload"))) 1.0 "None" true 1.0 0.0 false :!label _label_2)
              (:then
                (Variables|Default|SetAsync%20Task%20Reload _asynctaskproxy_2)
                (Utilities|FlowControl|Delay 0.3)
                (Class|GameplayAbility|ExecuteGameplayCuewithParams (Utilities|Struct|BreakProjectileParams (Variables|Default|GetCurrentProjectileParams)) (Ability|GameplayCue|MakeGameplayCueParameters :Instigator _returnvalue :EffectCauser _returnvalue)))
              (:OnBlendOut
                (Ability|EndAbility :!label _label_3))
              (:OnInterrupted
                (goto _label_3))
              (:OnCancelled
                (goto _label_3))))
          (:OnInterrupted
            (goto _label_2))
          (:OnCancelled
            (goto _label_2)))
        (else
          (goto _label_3))))
    (:False
      (goto _label))))

(event Ability|EventOnEndAbility
  (params (bWasCancelled :type Boolean))
  (CallFunction|CleanupAsyncTasks))

(fn CleanupAsyncTasks
  (bind _async_task_reload (Variables|Default|GetAsync%20Task%20Reload))
  (bind _async_task_fire (Variables|Default|GetAsync%20Task%20Fire))
  (Utilities|IsValid _async_task_reload
    (:Is%20Valid
      (GameplayTasks|EndTask _async_task_reload)
      (Utilities|IsValid _async_task_fire
        (:Is%20Valid
          (GameplayTasks|EndTask _async_task_fire))))))