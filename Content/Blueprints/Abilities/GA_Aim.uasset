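; Gameplay ability for aiming that lasts while its input is held.
; On activation it waits for input release and plays a rifle montage, applying the GE_Aim effect to the owner when the montage blends out.
; Input release or montage interruption or cancellation ends the ability.
; On end it removes the stored aim effect by handle and ends the input-release task.
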(event Ability|EventActivateAbility
  (bind _owningasc (Variables|Default|GetOwningASC))
  (bind _asynctaskproxy (Ability|Tasks|WaitInputRelease false)
    (:then
      (Variables|Default|SetWaitInputReleaseAsyncTask _asynctaskproxy)
      (|PlayMontageandWaitProxy "None" "/Game/Assets/Characters/Human/Male/Animations/LoadRifle__ID_106_variation_0__Montage.LoadRifle__ID_106_variation_0__Montage" 1.0 "None" true 1.0 0.0 false
        (:OnBlendOut
          (bind _returnvalue (GameplayEffects|ApplyGameplayEffectSpecToSelf _owningasc (GameplayEffects|MakeOutgoingSpec _owningasc "/Game/Blueprints/Abilities/GE_Aim.GE_Aim_C" 0.0 (GameplayEffects|MakeEffectContext _owningasc))))
          (Variables|Default|SetActiveAimEffect _returnvalue))
        (:OnInterrupted
          (Ability|EndAbility :!label _label))
        (:OnCancelled
          (goto _label))))
    (:OnRelease
      (goto _label))))

(event Ability|EventOnEndAbility
  (params (bWasCancelled :type Boolean))
  (Ability|RemoveGameplayEffectFromOwnerWithHandle (Variables|Default|GetActiveAimEffect))
  (CallFunction|CleanupAsyncTasks))

(fn CleanupAsyncTasks
  (bind _waitinputreleaseasynctask (Variables|Default|GetWaitInputReleaseAsyncTask))
  (Utilities|IsValid _waitinputreleaseasynctask
    (:Is%20Valid
      (GameplayTasks|EndTask _waitinputreleaseasynctask))))