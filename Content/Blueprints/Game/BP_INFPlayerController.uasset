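; BP_INFPlayerController is a player controller that toggles an inventory screen with the Tab key.
; A FlipFlop alternates between calling CreateInventoryWidget, with the cursor shown and Game and UI input, and closing the screen.
; Closing removes InventoryWidget from its parent, hides the cursor and restores game-only input, all only if the widget is valid.
; CreateInventoryWidget is not defined in this Blueprint's graphs, and the construction script is empty.
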(event Input|KeyboardEvents|Tab
  (params (Key :type Key%20Structure :default "None"))
  (bind _inventorywidget (Variables|Default|GetInventoryWidget))
  (:Pressed
    (Utilities|FlowControl|FlipFlop
      (:A
        (Class|INFPlayerController|CreateInventoryWidget)
        (Variables|Default|SetbShowMouseCursor true)
        (Input|SetInputModeGameandUI self 0 "DoNotLock" false false))
      (:B
        (Utilities|IsValid _inventorywidget
          (:Is%20Valid
            (Widget|RemovefromParent _inventorywidget)
            (Variables|Default|SetbShowMouseCursor false)
            (Input|SetInputModeGameOnly self false)))))))

(fn ConstructionScript)