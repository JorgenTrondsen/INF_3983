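; BP_INFPlayerState is a player state that carries a player's saved race, gender and model-part choices onto their character.
; On BeginPlay, remote instances and the authority instance whose controller name matches the first player controller load the "Appearance" save slot and call SR_UpdateAppearance.
; That event caches the pawn as BP_Character and stores the values; OnRep_ModelPartSelections then applies them through the character's UpdateAppearance.
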(event Custom|SR_UpdateAppearance
  (params (Race :type String) (Gender :type String) (ModelPartSelections :type Model%20Part%20Selection%20Data%20Structure))
  (bind _asbp_character (Utilities|Casting|CastToBP_Character (PlayerState|GetPawn)))
  (Variables|Default|SetBP_CharRef _asbp_character)
  (Variables|Default|SetRace Race)
  (Variables|Default|SetGender Gender)
  (Variables|Default|SetModelPartSelections ModelPartSelections))

(event EventBeginPlay
  (Networking|SwitchHasAuthority
    (:Authority
      (if (Utilities|Enum|Equal(Enum) (Utilities|String|ToString(Object) (Game|GetPlayerController)) "BP_INFPlayerController_C_0")
        (bind _returnvalue (SaveGame|LoadGamefromSlot "Appearance" :!label _label))
        (bind _asbp_ccsave (Utilities|Casting|CastToBP_CCSave _returnvalue))
        (CallFunction|SRUpdateAppearance (Variables|/Game/Blueprints/Player/BP_CCSave.BP_CCSave_C|GetRace _asbp_ccsave) (Variables|/Game/Blueprints/Player/BP_CCSave.BP_CCSave_C|GetGender _asbp_ccsave) (Variables|/Game/Blueprints/Player/BP_CCSave.BP_CCSave_C|GetModelPartSelections _asbp_ccsave))))
    (:Remote
      (goto _label))))

(fn ConstructionScript)

(fn OnRepModelPartSelections
  (Default|UpdateAppearance (Variables|Default|GetBP_CharRef) (Variables|Default|GetRace) (Variables|Default|GetGender) (Variables|Default|GetModelPartSelections)))