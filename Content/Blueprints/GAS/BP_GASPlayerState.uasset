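; Player state Blueprint that initializes a player character's appearance from race and gender.
; On BeginPlay, the authority waits briefly, then stores the pawn as InitAppearance, while non-authority instances load Race and Gender from the local "Appearance" save slot.
; The InitAppearance RepNotify passes its instance's Race and Gender to the character's UpdateAppearance, with no explicit wait for the save load.
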(event EventBeginPlay
  (Networking|SwitchHasAuthority
    (:Authority
      (Utilities|FlowControl|Delay 0.1)
      (bind _asbp_character (Utilities|Casting|CastToBP_Character (PlayerState|GetPawn)))
      (Variables|Default|SetInitAppearance _asbp_character))
    (:Remote
      (bind _returnvalue (SaveGame|LoadGamefromSlot "Appearance"))
      (bind _asbp_ccsave (Utilities|Casting|CastToBP_CCSave _returnvalue))
      (Variables|Default|SetRace (Variables|/Game/Blueprints/Player/BP_CCSave.BP_CCSave_C|GetRace _asbp_ccsave))
      (Variables|Default|SetGender (Variables|/Game/Blueprints/Player/BP_CCSave.BP_CCSave_C|GetGender _asbp_ccsave)))))

(fn ConstructionScript)

(fn OnRepInitAppearance
  (Default|UpdateAppearance (Variables|Default|GetInitAppearance) (Variables|Default|GetRace) (Variables|Default|GetGender)))