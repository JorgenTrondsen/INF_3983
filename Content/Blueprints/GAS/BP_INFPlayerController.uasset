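; Player controller Blueprint that binds hotkeys for projectile switching, item granting and the inventory screen.
; Key 1 flip-flops the dynamic projectile between two Projectile.Basic gameplay tags, and key 2 adds one random EquipmentItems entry to the InventoryComponent.
; Tab alternates between creating the inventory widget with cursor and Game And UI input, and removing it to restore Game Only input.
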(event Input|KeyboardEvents|1
  (params (Key :type Key%20Structure :default "None"))
  (:Pressed
    (Utilities|FlowControl|FlipFlop
      (:A
        (Class|INFAbilitySystemInterface|SetDynamicProjectile (GameplayTags|MakeLiteralGameplayTag "(TagName=\"Projectile.Basic.Type1\")")))
      (:B
        (Class|INFAbilitySystemInterface|SetDynamicProjectile (GameplayTags|MakeLiteralGameplayTag "(TagName=\"Projectile.Basic.Type2\")"))))))

(event Input|KeyboardEvents|Tab
  (params (Key :type Key%20Structure :default "None"))
  (bind _inventorywidget (Variables|Default|GetInventoryWidget))
  (:Pressed
    (Utilities|FlowControl|FlipFlop
      (:A
        (Class|INFPlayerController|CreateInventoryWidget)
        (Variables|Default|SetbShowMouseCursor true)
        (Input|SetInputModeGameandUI self 0 "DoNotLock" false false))
      (:B
        (Utilities|IsValid _inventorywidget
          (:Is%20Valid
            (Widget|RemovefromParent _inventorywidget)
            (Variables|Default|SetbShowMouseCursor false)
            (Input|SetInputModeGameOnly self false)))))))

(event Input|KeyboardEvents|2
  (params (Key :type Key%20Structure :default "None"))
  (:Pressed
    (Class|InventoryComponent|AddItem (Variables|Default|GetInventoryComponent) (.OutItem (Utilities|Array|Random (Variables|Default|GetEquipmentItems))) 1)))

(fn ConstructionScript)